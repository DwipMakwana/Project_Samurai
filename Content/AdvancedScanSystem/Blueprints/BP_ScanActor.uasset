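; Scan pulse actor that drives a post-process scan effect and detects tagged actors within its expanding radius, optionally following its origin actor.
; A delay-loop CustomTick macro advances progress to the scan curve's end time, then the actor destroys itself.
; Each update feeds position and progress to a dynamic material, adds a post-process component carrying it, and grows the overlap sphere.
; Overlapped actors matching TargetPoint tags spawn BP_AdvancedScan at their location.
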(event `self.ReceiveBeginPlay`
  (bind _scanstructure (`self.ScanStructure`))
  (bind _sphere (`self.Sphere`))
  (bind ((`ScanMaterialInstance_3_B404F42C4EFE593CD3CBB1998E96B7AF` _scanmaterialinstance) (`Curve_10_D8DD176C4CCFF025F9523A88485FAB72` _curve) (`ScanSpeed_13_DBB4DD134E5747DC6B72149E5F6EB946` _scanspeed) (`MaxRadius_15_175A36CC4614AA3B7F382DA86A584406` _maxradius) (`UseCameraPosition_67_204B945F42D2DE4934ABA88B24D3404B` _usecameraposition) (`ExcludeIndex_65_86158D2A483323AEBEF239BFADE27770` _excludeindex)) (break `/Game/AdvancedScanSystem/Blueprints/F_ScanStructure` _scanstructure))
  ;[0.125 0.125 0.125] Scan Logic
  (`self.UpdateOrigin` _scanstructure)
  (bind _returnvalue (`KismetMaterialLibrary.CreateDynamicMaterialInstance` _scanmaterialinstance))
  (`MaterialInstanceDynamic.SetScalarParameterValue` _returnvalue "UseCameraPosition" (select `bool` _usecameraposition :`false` 1.0 :!type "Float (single-precision)"))
  (`MaterialInstanceDynamic.SetScalarParameterValue` _returnvalue "ExcludeIndex" (`KismetMathLibrary.Conv_IntToDouble` _excludeindex))
  (`MaterialInstanceDynamic.SetScalarParameterValue` _returnvalue "MaxRadius" _maxradius)
  (bind (_return _intime) (`self.CustomTick` (`.MaxTime` (`CurveBase.GetTimeRange` _curve)) _scanspeed)
    (:`then`
      ;;[0.125 0.125 0.125] Spawn Target Point
      (add `PrimitiveComponent.OnComponentBeginOverlap` (`self.Sphere`) (delegate `Spawn Target Point`)))
    (:`Update`
      (`MaterialInstanceDynamic.SetVectorParameterValue` _returnvalue "Position" (`KismetMathLibrary.Conv_VectorToLinearColor` (`self.K2_GetActorLocation`)))
      (`MaterialInstanceDynamic.SetScalarParameterValue` _returnvalue "Progress" _intime)
      (bind _returnvalue_2 (`AddComponent|NODE_AddPostProcessComponent-0`))
      (set `PostProcessComponent.Settings` (make `PostProcessSettings` :`WeightedBlendables` (make `WeightedBlendables` (`|MakeArray` (make `WeightedBlendable` (select `bool` _return :`true` 1.0 :!type "Float (single-precision)") _returnvalue)))) _returnvalue_2)
      (`/Engine/EditorBlueprintResources/StandardMacros.IsValid` _sphere
        (:`Is Valid`
          (`SphereComponent.SetSphereRadius` _sphere (* _maxradius _intime) true))
        (:`Is Not Valid`
          (`self.K2_DestroyActor`))))
    (:`Done`
      (`self.K2_DestroyActor`))))

(event `Spawn Target Point`
  (params (OverlappedComponent :type "PrimitiveComponent Object Reference") (OtherActor :type "Actor Object Reference") (OtherComp :type "PrimitiveComponent Object Reference") (OtherBodyIndex :type Integer) (bFromSweep :type Boolean) (SweepResult :type "HitResult Structure (by ref)"))
  (bind _scanstructure (`self.ScanStructure`))
  ;[0.125 0.125 0.125] Scan Logic
  ;;[0.125 0.125 0.125] Spawn Target Point
  (for (_array_element _array_index) (`.TargetPoint_48_3D0DD93E47934280694486A43692F8B3` (break `/Game/AdvancedScanSystem/Blueprints/F_ScanStructure` _scanstructure))
    (if (`self.ActorHasTag` OtherActor (`.Tag_6_31B1680A43AEBFB89143489456A3D644` (break `/Game/AdvancedScanSystem/Blueprints/F_TargetPoint` _array_element)))
      (`|SpawnActorFromClass` "/Game/AdvancedScanSystem/Blueprints/BP_AdvancedScan.BP_AdvancedScan_C" (`KismetMathLibrary.MakeTransform` (`self.K2_GetActorLocation` OtherActor)) "AlwaysSpawn" "OverrideRootScale" null _scanstructure _array_index OtherComp (`self.OriginActor`) null))))

(fn `UserConstructionScript`)