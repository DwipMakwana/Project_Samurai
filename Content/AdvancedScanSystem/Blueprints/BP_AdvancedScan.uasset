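; Temporary scan marker actor that highlights a scanned object component and shows a target point widget with its distance.
; On BeginPlay it applies indexed settings from the current scan settings, styling the widget and enabling custom depth stencil on the object, optionally attaching to it.
; Tick shows meters from the first actor tagged as scan origin.
; After a delay it reverses the widget animation, disables the highlight and destroys itself.
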(event `Accept Settings`
  (bind _objectcomponent (`self.ObjectComponent`))
  (bind _as_wbp_target_point (`self.As WBP Target Point`))
  (bind ((`CustomDepth_27_A41C75474DAFF4CE37D3E2AC0F40DC6A` _customdepth) (`HightLightIndex_25_DA96E565470C4FCD308D509303E0F0DA` _hightlightindex) (`BackgroundColor_2_E2B450554552B6E238D324996BE5DA26` _backgroundcolor) (`StrokeColor_9_2575BB4D44E8C67682D066B4E7EC6765` _strokecolor) (`Text_22_68F7C77649D565DB3C3A87BCC7475374` _text) (`IconColor_33_E59B56E345D01D7E40630FBED4CE5BEE` _iconcolor) (`Icon_15_43747EA94A913B0E0B5C5BA8E1B00C22` _icon) (`IconSize_18_6F008CC641F4628B7BE524A127E3FB11` _iconsize)) (break `/Game/AdvancedScanSystem/Blueprints/F_TargetPoint` (`self.TargetPointSettings`)))
  (bind _icon_2 (`/Game/AdvancedScanSystem/Widgets/WBP_TargetPoint.Icon` _as_wbp_target_point))
  (bind _iconsize_2 (`/Game/AdvancedScanSystem/Widgets/WBP_TargetPoint.IconSize` _as_wbp_target_point))
  (bind (_x _y) (`KismetMathLibrary.BreakVector2D` _iconsize))
  ;[0.125 0.125 0.125] Accept Settings
  (`PrimitiveComponent.SetRenderCustomDepth` _objectcomponent _customdepth)
  (`PrimitiveComponent.SetCustomDepthStencilValue` _objectcomponent _hightlightindex)
  (`Border.SetBrushColor` _icon_2 _iconcolor)
  (`Border.SetBrushFromTexture` _icon_2 _icon)
  (`TextBlock.SetFont` (`/Game/AdvancedScanSystem/Widgets/WBP_TargetPoint.MeterText` _as_wbp_target_point) _text)
  (`Border.SetBrushColor` (`/Game/AdvancedScanSystem/Widgets/WBP_TargetPoint.Stroke` _as_wbp_target_point) _strokecolor)
  (`Border.SetBrushColor` (`/Game/AdvancedScanSystem/Widgets/WBP_TargetPoint.Background` _as_wbp_target_point) _backgroundcolor)
  (`SizeBox.SetHeightOverride` _iconsize_2 _x)
  (`SizeBox.SetHeightOverride` _iconsize_2 _y)
  (`self.LiveUpdate`))

(event `self.ReceiveBeginPlay`
  (bind _as_wbp_target_point (`self.As WBP Target Point`))
  ;[0.125 0.125 0.125] Import Settings from Data Table
  (bind _aswbp_target_point (cast `/Game/AdvancedScanSystem/Widgets/WBP_TargetPoint` (`WidgetComponent.GetUserWidgetObject` (`self.TargetPoint`))))
  (set `self.As WBP Target Point` _aswbp_target_point)
  (set `self.TargetPointSettings` (`|GetArrayItem` (`.TargetPoint_48_3D0DD93E47934280694486A43692F8B3` (break `/Game/AdvancedScanSystem/Blueprints/F_ScanStructure` (`self.CurrentScanSettings`))) (`self.Index`)))
  (`self.Accept Settings`)
  (`/Game/AdvancedScanSystem/Widgets/WBP_TargetPoint.Play Animation` _as_wbp_target_point "Forward" 1.0 0.0)
  (`KismetSystemLibrary.Delay` (`.Delay_21_B0EB87F046BEBB39BBDBC7B89608F614` (break `/Game/AdvancedScanSystem/Blueprints/F_TargetPoint` (`self.TargetPointSettings`))))
  (`/Game/AdvancedScanSystem/Widgets/WBP_TargetPoint.Play Animation` _as_wbp_target_point "Reverse" 1.0 0.0)
  (`KismetSystemLibrary.Delay` 0.25)
  (`PrimitiveComponent.SetRenderCustomDepth` (`self.ObjectComponent`) false)
  (`self.K2_DestroyActor`))

(event `self.ReceiveTick`
  (params (DeltaSeconds :type "Float (single-precision)"))
  ;[0.125 0.125 0.125] Calculate Meter
  (bind _outactors (`GameplayStatics.GetAllActorsOfClassWithTag` "/Script/Engine.Actor" (`.ScanOrigin_53_06EA5E284F2EC46799E941BAB3F88C78` (break `/Game/AdvancedScanSystem/Blueprints/F_ScanStructure` (`self.CurrentScanSettings`)))))
  (bind _output (`|GetArrayItem` _outactors))
  (`/Engine/EditorBlueprintResources/StandardMacros.IsValid` _output
    (:`Is Valid`
      (`TextBlock.SetText` (`/Game/AdvancedScanSystem/Widgets/WBP_TargetPoint.MeterText` (`self.As WBP Target Point`)) (`KismetTextLibrary.Conv_StringToText` (`KismetStringLibrary.Concat_StrStr` (`KismetTextLibrary.Conv_TextToString` (`KismetTextLibrary.Conv_IntToText` (`KismetMathLibrary.FTrunc` (/ (`KismetMathLibrary.Vector_Distance` (`self.K2_GetActorLocation` _output) (`self.K2_GetActorLocation`)) 100.0)))) "M"))))))

(event `LiveUpdate`
  ;[0.125 0.125 0.125] Live Update
  (if (`.LiveUpdate_39_744904F041822925E0C64DB10492AF1E` (break `/Game/AdvancedScanSystem/Blueprints/F_TargetPoint` (`self.TargetPointSettings`)))
    (`self.K2_AttachToComponent` (`self.ObjectComponent`) "None" "KeepWorld" "KeepWorld" "KeepWorld")))

(fn `UserConstructionScript`)