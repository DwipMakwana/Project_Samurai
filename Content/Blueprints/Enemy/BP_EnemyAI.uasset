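; Samurai enemy character that fights the player with melee combos, dodges and lunging special attacks, and can be assassinated before it draws its weapon.
; BeginPlay runs BT_EnemyAI, feeds its blackboard and starts random-interval timers for defence, strafing and optional specials.
; Sphere traces deal damage, while incoming hits respect dodge and guard, with special attacks breaking guard.
; Health changes drive a lagging health bar, and death triggers a Niagara dissolve before destroying the actor.
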(event `self.ReceiveTick`
  (params (DeltaSeconds :type "Float (single-precision)"))
  ;[1 1 1] EventTick
  (if (and (not (`self.isDead`)) (`self.Equip`))
    (`self.K2_SetActorRotation` (`KismetMathLibrary.RInterpTo` (`self.K2_GetActorRotation`) (`KismetMathLibrary.FindLookAtRotation` (`self.K2_GetActorLocation`) (`self.K2_GetActorLocation` (`self.PlayerTarget`))) (`GameplayStatics.GetWorldDeltaSeconds`) 25.0))
    (`self.AddMovementInput` (`self.GetActorRightVector`) (`self.Strafe Value`))))

(event `self.ReceiveBeginPlay`
  ;[1 1 1] EventBeginPlay
  (`|ExecutionSequence`
    (:`then_0`
      (bind _aswbp_enemy_health_bar (cast `/Game/Blueprints/Player/UI/WBP_EnemyHealthBar` (`WidgetComponent.GetWidget` (`self.HealthWidget`))))
      (set `self.Health Bar Widget` _aswbp_enemy_health_bar)
      (bind _aswbp_assassinate_widget (cast `/Game/Blueprints/Player/UI/WBP_AssassinateWidget` (`WidgetComponent.GetWidget` (`self.AssassinationWidget`))))
      (set `self.Assassination Widget` _aswbp_assassinate_widget)
      (`self.IncreaseHealth` (/ (`self.Current Health`) (`self.Max Health`)))
      (bind _asabp_enemy_ai (cast `/Game/Blueprints/Enemy/ABP_EnemyAI` (`SkeletalMeshComponent.GetAnimInstance` (`self.Mesh`))))
      (set `self.ABP Enemy AI` _asabp_enemy_ai)
      (bind _asabp_enemy_ai_2 (cast `/Game/Blueprints/Enemy/ABP_EnemyAI` (`SkeletalMeshComponent.GetAnimInstance` (`self.Mesh`))))
      (set `self.ABP Enemy AI` _asabp_enemy_ai_2)
      (`AIController.RunBehaviorTree` (`AIBlueprintHelperLibrary.GetAIController` self) "/Game/Blueprints/Enemy/BB_BT/BT_EnemyAI.BT_EnemyAI")
      (bind _returnvalue (`GameplayStatics.GetActorOfClass` "/Game/Blueprints/Player/BP_Player.BP_Player_C"))
      (bind _output_get (set `self.PlayerTarget` _returnvalue))
      (`BlackboardComponent.SetValueAsObject` (`AIBlueprintHelperLibrary.GetBlackboard` self) "Target" _output_get)
      (`BlackboardComponent.SetValueAsVector` (`AIBlueprintHelperLibrary.GetBlackboard` self) "RandomLocation" (`self.temp_move_loc`)))
    (:`then_1`
      ;[1 1 1] Timer Handles
      (`KismetSystemLibrary.K2_SetTimerDelegate` (delegate `SetDefense`) (`KismetMathLibrary.RandomFloatInRange` 15.0 20.0) true))
    (:`then_2`
      (`KismetSystemLibrary.K2_SetTimerDelegate` (delegate `SetStrafe`) (`KismetMathLibrary.RandomFloatInRange` 10.0 15.0) true))
    (:`then_3`
      (if (`self.Special Attack`)
        (`KismetSystemLibrary.K2_SetTimerDelegate` (delegate `SpecialAttack`) (`KismetMathLibrary.RandomFloatInRange` 5.0 10.0) true)))))

(event `StorePlayerLocation`
  (bind (_returnvalue_x _returnvalue_y _returnvalue_z) (`KismetMathLibrary.BreakVector` (`self.K2_GetActorLocation` (`self.PlayerTarget`))))
  ;[1 1 1] Store Player Location
  (bind _output_get (set `self.Target Location` (`KismetMathLibrary.MakeVector` _returnvalue_x _returnvalue_y _returnvalue_z))))

(event `SpecialAttack`
  (bind (_returnvalue_x _returnvalue_y) (`KismetMathLibrary.BreakVector` (`self.GetActorForwardVector`)))
  ;[1 1 1] Timer Handles
  (if (and (`self.Equip`) (not (`self.isDead`)))
    (set `self.Attacking` true)
    (if (`KismetMathLibrary.RandomBool`)
      (`self.PlayAnimMontage` "/Game/Animations/GhostSamurai_Katana/GhostSamurai_Katana/Animation/Apose/Attack/Root/GhostSamurai_APose_JumpAttack02_Root_Montage.GhostSamurai_APose_JumpAttack02_Root_Montage")
      (`self.LaunchCharacter` (`KismetMathLibrary.MakeVector` _returnvalue_x _returnvalue_y 1000.0))
      (`KismetSystemLibrary.Delay` 0.5)
      (`self.StorePlayerLocation`)
      (bind (_direction _alpha) (`Timeline|SpecialAttackJumpTimeline` :!via `PlayFromStart`)
        (:`Update`
          (`self.K2_SetActorLocation` (`KismetMathLibrary.VLerp` (`self.K2_GetActorLocation`) (`self.Target Location`) _alpha) true)))
      (else
        (`self.PlayAnimMontage` "/Game/Animations/GhostSamurai_Katana/GhostSamurai_Katana/Animation/Apose/Attack/Root/GhostSamurai_APose_SPAttack01_Root_Montage.GhostSamurai_APose_SPAttack01_Root_Montage")
        (`KismetSystemLibrary.Delay` 1.1)
        (`self.StorePlayerLocation`)
        (bind (_direction_2 _alpha_2) (`Timeline|SpecialAttackSwooshTimeline` :!via `PlayFromStart`)
          (:`Update`
            (`self.K2_SetActorLocation` (`KismetMathLibrary.VLerp` (`self.K2_GetActorLocation`) (`self.Target Location`) _alpha_2) true)))))))

(event `SetStrafe`
  ;[1 1 1] Timer Handles
  (if (not (`self.isDead`))
    (set `self.Strafe` true)
    (`BlackboardComponent.SetValueAsBool` (`AIBlueprintHelperLibrary.GetBlackboard` self) "Strafe" true)))

(event `SetDefense`
  ;[1 1 1] Timer Handles
  (if (not (`self.isDead`))
    (`self.Sprint` false)
    (set `self.Defence` true)
    (`KismetSystemLibrary.Delay` (`KismetMathLibrary.RandomFloatInRange` 5.0 10.0))
    (set `self.Defence` false)))

(event `Sprint`
  (params (status :type Boolean))
  ;[1 1 1] Sprint
  (bind _output_get (set `self.Sprinting` status))
  (if _output_get
    (bind (_direction _unequippedsprintvalue _equippedsprintvalue) (`Timeline|SprintTimeline` :!label _label)
      (:`Update`
        (set `CharacterMovementComponent.MaxWalkSpeed` (`KismetMathLibrary.SelectFloat` _equippedsprintvalue _unequippedsprintvalue (`self.Equip`)) (`self.CharacterMovement`))))
    (else
      (goto _label :!via `Reverse`))))

(event `PlayNiagaraFX`
  (params (SystemTemplate :type "NiagaraSystem Object Reference") (SpawnLocation :type "Vector Structure") (SpawnRotation :type "Rotator Structure"))
  ;[1 1 1] NiagaraFx
  (`NiagaraFunctionLibrary.SpawnSystemAtLocation` SystemTemplate SpawnLocation SpawnRotation))

(event `Attack`
  ;[1 1 1] Attack
  (if (not (or (`self.Attacking`) (`self.IsHit`) (`self.isDead`)))
    (set `self.Attacking` true)
    (if (== (`KismetMathLibrary.RandomIntegerInRange` 0 6) 0)
      (set `self.Dodge` true)
      (`self.PlayAnimMontage` null)
      (else
        (`self.PlayAnimMontage` (`|GetArrayItem` (`self.Atack Anim Montages`) (`KismetMathLibrary.RandomIntegerInRange` 0 4)))))))

(event `SetHealthPercentLag`
  (params (TargetHealth :type "Float (double-precision)"))
  (bind _max_health (`self.Max Health`))
  (bind _backhealthbarlag (`/Game/Blueprints/Player/UI/WBP_EnemyHealthBar.BackHealthBarLag` (`self.Health Bar Widget`)))
  ;[1 1 1] HealthBarAnim
  (bind _value (`self.FloatTimeline` "/Game/Blueprints/Player/Curves/LinearCurve.LinearCurve")
    (:`Out`
      (`ProgressBar.SetPercent` _backhealthbarlag (/ (`KismetMathLibrary.Lerp` (* (`ProgressBar.Percent` _backhealthbarlag) _max_health) TargetHealth _value) _max_health)))))

(event `ResetAttack`
  ;[1 1 1] Attack
  (set `self.Attacking` false)
  (set `self.Dodge` false))

(event `ToggleLockTarget`
  (params (Lock :type Boolean))
  ;[1 1 1] Toggle Lock Target
  (`SceneComponent.SetVisibility` (`self.TargetLockWidget`) Lock false))

(event `AttackSphere`
  (params (SpecialAttack :type Boolean))
  (bind _attackarrow (`self.AttackArrow`))
  (bind _returnvalue (`SceneComponent.K2_GetComponentLocation` _attackarrow))
  ;[1 1 1] Attack Sphere (Do Damage)
  (bind (_outhits _returnvalue_2) (`KismetSystemLibrary.SphereTraceMulti` :`Start` _returnvalue :`End` (+ _returnvalue (* (`SceneComponent.GetForwardVector` _attackarrow) 150.0)) :`Radius` 50.0 :`TraceChannel` "TraceTypeQuery1" :`DrawTime` 2.0))
  (if _returnvalue_2
    (for _array_element _outhits
      (bind (_bblockinghit _binitialoverlap _time _distance _location _impactpoint _normal _impactnormal _physmat _hitactor) (`GameplayStatics.BreakHitResult` _array_element))
      (bind _asbp_player (cast `/Game/Blueprints/Player/BP_Player` _hitactor))
      (`/Game/Blueprints/Player/BP_Player.Damage` _asbp_player 20.0 SpecialAttack _location (`KismetMathLibrary.MakeRotFromXY` _impactpoint _impactpoint) false 0))))

(event `self.Ready`
  (params (Equip :type Boolean))
  ;[1 1 1] EventReady
  (if (not (or (`self.isDead`) (`self.Equip`) (`self.IsAssassinated`)))
    (`SceneComponent.SetVisibility` (`self.AssassinationWidget`) false false)
    (bind _output_get (set `self.Equip` Equip))
    (`self.PlayAnimMontage` (select `bool` _output_get :`false` "/Game/Animations/GhostSamurai_Katana/GhostSamurai_Katana/Animation/Common/Root/GhostSamurai_APose_Unarm_1_Root_Montage.GhostSamurai_APose_Unarm_1_Root_Montage" :`true` "/Game/Animations/GhostSamurai_Katana/GhostSamurai_Katana/Animation/Common/Root/GhostSamurai_APose_Equip02_Root_Montage.GhostSamurai_APose_Equip02_Root_Montage" :!type "AnimMontage Object Reference"))
    (`KismetSystemLibrary.Delay` 2.0)
    (`BlackboardComponent.SetValueAsBool` (`AIBlueprintHelperLibrary.GetBlackboard` self) "ReadyToFight" _output_get)
    (set `self.CanBeAssassinated` false)))

(event `/Game/Blueprints/Player/Interfaces/BPI_Damage.Damage`
  (params (Damage :type "Float (double-precision)") (SpecialAttack :type Boolean) (HitLocation :type "Vector Structure") (HitRotation :type "Rotator Structure") (Assassination :type Boolean) (`Assassination Montage Index` :type Integer))
  (bind _defence (`self.Defence`))
  ;[1 1 1] Take Damage
  (set `self.Attacking` false)
  (if (not (`self.Dodge`))
    (set `self.IsHit` true)
    (if Assassination
      (bind _isdead (`self.DecreaseHealth` Damage :!label _label_2))
      (if _isdead
        (set `self.CanBeAssassinated` false)
        (set `self.Assassinate Anim Index` `Assassination Montage Index`)
        (set `self.IsAssassinated` true)
        (`self.Die` Assassination `Assassination Montage Index` :!label _label_3)
        (else
          (`self.PlayAnimMontage` "/Game/Animations/GhostSamurai_Katana/GhostSamurai_Katana/Animation/Apose/Hit/Root/GhostSamurai_APose_Hit_F_Root_Montage.GhostSamurai_APose_Hit_F_Root_Montage")
          (`KismetSystemLibrary.Delay` 0.5)
          (set `self.IsHit` false :!label _label_4)))
      (else
        (`self.PlayNiagaraFX` "/Game/FX/Realistic_Starter_VFX_Pack_Niagara/Niagara/Impact/NS_Impact_SwordClash.NS_Impact_SwordClash" HitLocation HitRotation)
        (if SpecialAttack
          (if _defence
            (`self.PlayAnimMontage` "/Game/Animations/GhostSamurai_Katana/GhostSamurai_Katana/Animation/Defense/Root/GhostSamurai_DefenseR_Broken_Root_Montage.GhostSamurai_DefenseR_Broken_Root_Montage")
            (else
              (bind _isdead_2 (`self.DecreaseHealth` Damage))
              (if _isdead_2
                (goto _label_3)
                (else
                  (`self.PlayAnimMontage` "/Game/Animations/GhostSamurai_Katana/GhostSamurai_Katana/Animation/Apose/Hit/Root/GhostSamurai_APose_Large_Hit_Root_Montage.GhostSamurai_APose_Large_Hit_Root_Montage")))))
          (`KismetSystemLibrary.Delay` 1.0)
          (goto _label_4)
          (elif _defence
            (`self.PlayAnimMontage` "/Game/Animations/GhostSamurai_Katana/GhostSamurai_Katana/Animation/Defense/Root/GhostSamurai_DefenseL_Hit01_Root_Montage.GhostSamurai_DefenseL_Hit01_Root_Montage")
            (`KismetSystemLibrary.Delay` 1.0)
            (set `self.IsHit` false)
            (else
              (goto _label_2))))))))

(event `DieFX`
  (bind _dieparticles (`self.DieParticles`))
  (bind _mesh (`self.Mesh`))
  (bind _returnvalue (select `bool` (`|EnumEquality` (`self.EnemyType`) "NewEnumerator0") :`false` "/Game/FX/Edge_Dissolve/M_DissolveRed.M_DissolveRed" :`true` "/Game/FX/Edge_Dissolve/M_Dissolve.M_Dissolve" :!type "MaterialInterface Object Reference"))
  ;[1 1 1] DieFX
  (`PrimitiveComponent.CreateDynamicMaterialInstance` _mesh 0 (`PrimitiveComponent.GetMaterial` _mesh 0) "None")
  (`PrimitiveComponent.SetMaterial` _mesh 0 _returnvalue)
  (`PrimitiveComponent.CreateDynamicMaterialInstance` _mesh 1 (`PrimitiveComponent.GetMaterial` _mesh 1) "None")
  (`PrimitiveComponent.SetMaterial` _mesh 1 _returnvalue)
  (`SceneComponent.SetVisibility` (`self.DieParticles`) true false)
  (bind (_direction _particleanim _noisedragnaim) (`Timeline|ParticlesTimeline` :!via `PlayFromStart`)
    (:`Update`
      (`MeshComponent.SetScalarParameterValueOnMaterials` (`self.Mesh`) "Animation" _particleanim)
      (`NiagaraComponent.SetVariableFloat` _dieparticles "User_Noise" _noisedragnaim)
      (`NiagaraComponent.SetVariableFloat` _dieparticles "User_Animation" _particleanim)
      (if (and (> _particleanim 0.3) (not (`self.isDestroyed`)))
        (`ActorComponent.K2_DestroyComponent` (`self.Bracelet`))
        (`ActorComponent.K2_DestroyComponent` (`self.Hat`))
        (`ActorComponent.K2_DestroyComponent` (`self.Scabbard`))
        (`ActorComponent.K2_DestroyComponent` (`self.Katana`))
        (set `self.isDestroyed` true)))
    (:`Finished`
      (`KismetSystemLibrary.Delay` 2.0)
      (`self.K2_DestroyActor`))))

(event `self.NearOverlap.OnComponentBeginOverlap`
  (params (OverlappedComponent :type "PrimitiveComponent Object Reference") (OtherActor :type "Actor Object Reference") (OtherComp :type "PrimitiveComponent Object Reference") (OtherBodyIndex :type Integer) (bFromSweep :type Boolean) (SweepResult :type "HitResult Structure (by ref)"))
  ;[1 1 1] Toggle Vicinity UI
  (if (and (`self.ActorHasTag` OtherActor "Player") (not (`self.isDead`)))
    _))

(event `Die`
  (params (Aassinated :type Boolean) (`Assassinate Index` :type Integer))
  (bind _returnvalue (`AIBlueprintHelperLibrary.GetBlackboard` null))
  (bind _playertarget (`self.PlayerTarget`))
  ;[1 1 1] Die
  (`self.StopAnimMontage` (`self.GetCurrentMontage`))
  (`self.ResetAttack`)
  (`BlackboardComponent.SetValueAsBool` _returnvalue "isDead" true)
  (`BlackboardComponent.SetValueAsBool` _returnvalue "ReadyToFight" false)
  (if (`/Game/Blueprints/Player/BP_Player.Lock` _playertarget)
    (`/Game/Blueprints/Player/BP_Player.UnlockTarget` _playertarget))
  (set `self.DeathAnimIndex` (`KismetMathLibrary.RandomIntegerInRange` 0 10))
  (`PrimitiveComponent.SetCollisionEnabled` (`self.CapsuleComponent`) "NoCollision")
  (`PrimitiveComponent.SetCollisionEnabled` (`self.Mesh`) "NoCollision")
  (`PrimitiveComponent.SetCollisionEnabled` (`self.Katana`) "NoCollision")
  (`PrimitiveComponent.SetCollisionEnabled` (`self.Bracelet`) "NoCollision")
  (`PrimitiveComponent.SetCollisionEnabled` (`self.Scabbard`) "NoCollision")
  (`PrimitiveComponent.SetCollisionEnabled` (`self.Hat`) "NoCollision")
  (`SceneComponent.SetVisibility` (`self.HealthWidget`) false false)
  (`SceneComponent.SetVisibility` (`self.AssassinationWidget`) false false)
  (if Aassinated
    (`KismetSystemLibrary.Delay` (`KismetMathLibrary.SelectFloat` 3.0 2.0 (> `Assassinate Index` 2))))
  (set `self.isDead` true)
  (`self.DieFX`))

(event `self.NearOverlap.OnComponentEndOverlap`
  (params (OverlappedComponent :type "PrimitiveComponent Object Reference") (OtherActor :type "Actor Object Reference") (OtherComp :type "PrimitiveComponent Object Reference") (OtherBodyIndex :type Integer))
  ;[1 1 1] Toggle Vicinity UI
  (if (`self.ActorHasTag` OtherActor "Player")
    (`SceneComponent.SetVisibility` (`self.TargetLockWidget`) false false :!label _label_5)
    (`SceneComponent.SetVisibility` (`self.AssassinationWidget`) false false)
    (set `self.CanBeAssassinated` false)
    (`Widget.SetVisibility` (`/Game/Blueprints/Player/UI/WBP_EnemyHealthBar.AssDmgHealthBar` (`self.Health Bar Widget`)) "Hidden")))

(event `Toggle Widgets`
  (params (`health widget` :type Boolean) (`ass widget` :type Boolean))
  ;[1 1 1] Toggle Vicinity UI
  (if `health widget`
    (if (not (`self.Equip`))
      (set `self.CanBeAssassinated` true)
      (if (not (`self.IsAssassinated`))
        (if `ass widget`
          (`SceneComponent.SetVisibility` (`self.AssassinationWidget`) true false)
          (`Widget.SetVisibility` (`/Game/Blueprints/Player/UI/WBP_EnemyHealthBar.AssDmgHealthBar` (`self.Health Bar Widget`)) "Visible")
          (`self.Set Assassination Damage`))))
    (else
      (goto _label_5))))

(fn `Assassinate`
  (returns (`Front Ref Location` :type "Vector Structure") (`Back Ref Location` :type "Vector Structure") (`Ref Rotation` :type "Rotator Structure"))
  (return (`SceneComponent.K2_GetComponentLocation` (`self.AssassinRefFront`)) (`SceneComponent.K2_GetComponentLocation` (`self.AssassinRefBack`)) (`self.K2_GetActorRotation`)))

(fn `Check Enemy Distaance`
  (bind _health_bar_widget (`self.Health Bar Widget`))
  (bind _playertarget (`self.PlayerTarget`)
    (:`then`
      (bind _returnvalue (`self.K2_GetActorLocation` _playertarget))
      (if (< (`KismetMathLibrary.Vector_Distance` _returnvalue _returnvalue) 1000.0)
        (`Widget.SetVisibility` _health_bar_widget "Visible")
        (else
          (`Widget.SetVisibility` _health_bar_widget "Hidden"))))
    (:`else`)))

(fn `Check Player Distance`
  (bind _playertarget (`self.PlayerTarget`)
    (:`then`
      (`KismetSystemLibrary.PrintString` (`KismetStringLibrary.Conv_DoubleToString` (`KismetMathLibrary.Vector_Distance` (`self.K2_GetActorLocation` _playertarget) (`self.K2_GetActorLocation`)))))
    (:`else`)))

(fn `DecreaseHealth`
  (params (Damage :type "Float (double-precision)"))
  (returns (isDead :type Boolean))
  (bind _health_bar_widget (`self.Health Bar Widget`))
  (bind _max_health (`self.Max Health`))
  (bind _returnvalue (- (`self.Current Health`) Damage))
  (bind _fronthealthbar (`/Game/Blueprints/Player/UI/WBP_EnemyHealthBar.FrontHealthBar` _health_bar_widget))
  (bind _healthtext (`/Game/Blueprints/Player/UI/WBP_EnemyHealthBar.HealthText` _health_bar_widget))
  (if (<= _returnvalue 0.0)
    (bind _output_get (set `self.Current Health` 0.0))
    (`ProgressBar.SetPercent` _fronthealthbar (/ _output_get _max_health))
    (`TextBlock.SetText` _healthtext "")
    (`self.SetHealthPercentLag` 0.0)
    (return true)
    (else
      (bind _output_get_2 (set `self.Current Health` _returnvalue))
      (`ProgressBar.SetPercent` _fronthealthbar (/ _output_get_2 _max_health))
      (`TextBlock.SetText` _healthtext (`KismetTextLibrary.Conv_DoubleToText` _output_get_2 "HalfToEven"))
      (`self.SetHealthPercentLag` _output_get_2)
      (return false))))

(fn `IncreaseHealth`
  (params (Health :type "Float (double-precision)"))
  (bind _max_health (`self.Max Health`))
  (bind _max_health_2 (`self.Max Health`))
  (bind _health_bar_widget (`self.Health Bar Widget`))
  (bind _returnvalue (+ Health (`self.Current Health`)))
  (bind _fronthealthbar (`/Game/Blueprints/Player/UI/WBP_EnemyHealthBar.FrontHealthBar` _health_bar_widget))
  (bind _backhealthbarlag (`/Game/Blueprints/Player/UI/WBP_EnemyHealthBar.BackHealthBarLag` _health_bar_widget))
  (bind _healthtext (`/Game/Blueprints/Player/UI/WBP_EnemyHealthBar.HealthText` _health_bar_widget))
  (if (> _returnvalue _max_health)
    (bind _output_get (set `self.Current Health` _max_health))
    (bind _returnvalue_2 (/ _output_get _max_health_2))
    (`ProgressBar.SetPercent` _fronthealthbar _returnvalue_2)
    (`TextBlock.SetText` _healthtext (`KismetTextLibrary.Conv_DoubleToText` _output_get "HalfToEven"))
    (`ProgressBar.SetPercent` _backhealthbarlag _returnvalue_2)
    (else
      (bind _output_get_2 (set `self.Current Health` _returnvalue))
      (bind _returnvalue_3 (/ _output_get_2 _max_health_2))
      (`ProgressBar.SetPercent` _fronthealthbar _returnvalue_3)
      (`TextBlock.SetText` _healthtext (`KismetTextLibrary.Conv_DoubleToText` _output_get_2 "HalfToEven"))
      (`ProgressBar.SetPercent` _backhealthbarlag _returnvalue_3)))
  (return))

(fn `Set Assassination Damage`
  (bind _playertarget (`self.PlayerTarget`)
    (:`then`
      (`ProgressBar.SetPercent` (`/Game/Blueprints/Player/UI/WBP_EnemyHealthBar.AssDmgHealthBar` (`self.Health Bar Widget`)) (/ (`/Game/Blueprints/Player/BP_Player.Assassination Damage` _playertarget) (`self.Max Health`))))
    (:`else`)))

(fn `UserConstructionScript`)