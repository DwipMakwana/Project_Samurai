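; Base player character for melee combat against BP_EnemyAI, with equip, sprint, crouch, parry, sway/dodge and randomized montage attacks.
; State booleans gate each action, and a repeated directional dodge press within half a second turns a sway into a dodge.
; Lock-on steers control rotation toward the nearest enemy, while AttackSphere sphere-traces to damage enemies.
; Incoming damage plays guard or hit reactions unless dodging, with camera shake and a post-process pulse for special attacks.
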(event `InputAxis|Mouse X`
  (params (AxisValue :type "Float (single-precision)"))
  ;[1 1 1] Camera Movement
  (if (not (`self.Lock`))
    (`self.AddControllerYawInput` AxisValue)))

(event `InputAxis|Mouse Y`
  (params (AxisValue :type "Float (single-precision)"))
  ;[1 1 1] Camera Movement
  (if (not (`self.Lock`))
    (`self.AddControllerPitchInput` AxisValue)))

(event `InputAction|Equip`
  (params (Key :type "Key Structure"))
  (bind _equip (`self.Equip`))
  ;[1 1 1] Equip
  (:`Pressed`
    (if (`self.Crouched`)
      _
      (elif _equip
        (set `self.Equip` false)
        (`self.PlayAnimMontage` "/Game/GhostSamurai_Katana/GhostSamurai_Katana/Animation/Common/Root/GhostSamurai_APose_Unarm_1_Root_Montage.GhostSamurai_APose_Unarm_1_Root_Montage")
        (`KismetSystemLibrary.Delay` 1.0)
        (else
          (set `self.Equip` true)
          (`self.PlayAnimMontage` "/Game/GhostSamurai_Katana/GhostSamurai_Katana/Animation/Common/Root/GhostSamurai_APose_Equip02_Root_Montage.GhostSamurai_APose_Equip02_Root_Montage")
          (`KismetSystemLibrary.Delay` 1.0)
          (message `/Game/BP_WorldSettings/BPI_ReadyToFight.Ready` (`self.Target`) _equip))))))

(event `InputAxis|MoveFwd`
  (params (AxisValue :type "Float (single-precision)"))
  ;[1 1 1] Player Movement
  (`self.AddMovementInput` (`KismetMathLibrary.GetForwardVector` (`KismetMathLibrary.MakeRotator` 0.0 0.0 (.yaw (`self.GetControlRotation`)))) AxisValue))

(event `InputAxis|MoveRight`
  (params (AxisValue :type "Float (single-precision)"))
  ;[1 1 1] Player Movement
  (`self.AddMovementInput` (`KismetMathLibrary.GetRightVector` (`KismetMathLibrary.MakeRotator` 0.0 0.0 (.yaw (`self.GetControlRotation`)))) AxisValue))

(event `InputAction|Sprint`
  (params (Key :type "Key Structure"))
  ;[1 1 1] Sprint
  (:`Pressed`
    (if (not (or (`self.Defend`) (`self.Crouched`)))
      (set `self.Sprint` true)
      (bind (_direction _sprintvalue) (`Timeline|SprintTimeline` :!label _label)
        (:`Update`
          (set `CharacterMovementComponent.MaxWalkSpeed` _sprintvalue (`self.CharacterMovement`))))))
  (:`Released`
    (set `self.Sprint` false :!label _label_2)
    (goto _label :!via `Reverse`)))

(event `InputAction|Crouch`
  (params (Key :type "Key Structure"))
  ;[1 1 1] Crouch
  (:`Pressed`
    (if (not (or (`self.Equip`) (`self.Sprint`)))
      (`/Engine/EditorBlueprintResources/StandardMacros.FlipFlop`
        (:`A`
          (set `self.Crouched` true))
        (:`B`
          (set `self.Crouched` false))))))

(event `InputAction|Defend`
  (params (Key :type "Key Structure"))
  ;[1 1 1] Parry
  (:`Pressed`
    (if (`self.Equip`)
      (`|ExecutionSequence`
        (:`then_0`
          (goto _label_2))
        (:`then_1`
          (set `self.Defend` true)))))
  (:`Released`
    (set `self.Defend` false)))

(event `ResetSway`
  ;[1 1 1] Dodge
  (set `self.Sway` false))

(event `InputAction|Dodge`
  (params (Key :type "Key Structure"))
  (bind _returnvalue (`self.GetInputAxisValue`))
  (bind _returnvalue_2 (`self.GetInputAxisValue`))
  (bind _dodge (`self.Dodge`))
  (bind _dodge_2 (`self.Dodge`))
  ;[1 1 1] Dodge
  (:`Pressed`
    (if (or (`self.Dodge`) (`self.Attack`) (`self.Is Hit`))
      _
      (elif (`self.Equip`)
        (`|ExecutionSequence`
          (:`then_0`
            (if (!= _returnvalue_2 0.0)
              (if (`self.Sway`)
                (set `self.Sway` false)
                (set `self.Dodge` true)
                (else
                  (set `self.Sway` true)
                  (set `self.Dodge` false)
                  (`KismetSystemLibrary.K2_SetTimerDelegate` (delegate `ResetSway`) 0.5)))
              (if (>= _returnvalue_2 0.0)
                (`self.PlayAnimMontage` (select `bool` _dodge_2 :`false` "/Game/GhostSamurai_Katana/GhostSamurai_Katana/Animation/Apose/Dodge/Root/GhostSamurai_APose_Avoid_F_Root_Montage.GhostSamurai_APose_Avoid_F_Root_Montage" :`true` "/Game/GhostSamurai_Katana/GhostSamurai_Katana/Animation/Apose/Dodge/Root/GhostSamurai_APose_Dodge_F_Root_Montage.GhostSamurai_APose_Dodge_F_Root_Montage" :!type "AnimMontage Object Reference") 1.5)
                (else
                  (`self.PlayAnimMontage` (select `bool` _dodge_2 :`false` (`KismetArrayLibrary.Array_Random` (`self.Back Sway`)) :`true` (`KismetArrayLibrary.Array_Random` (`self.Back Dodge`))) 1.5)))
              (if (`self.Dodge`) :!label _label_3
                (`KismetSystemLibrary.Delay` 1.0))
              (set `self.Dodge` false)
              (elif (!= _returnvalue 0.0)
                (if (`self.Sway`)
                  (set `self.Sway` false)
                  (set `self.Dodge` true)
                  (else
                    (set `self.Sway` true)
                    (set `self.Dodge` false)
                    (`KismetSystemLibrary.K2_SetTimerDelegate` (delegate `ResetSway`) 0.5)))
                (if (>= _returnvalue 0.0)
                  (`self.PlayAnimMontage` (select `bool` _dodge :`false` (`KismetArrayLibrary.Array_Random` (`self.Right Sway`)) :`true` "/Game/GhostSamurai_Katana/GhostSamurai_Katana/Animation/Apose/Dodge/Root/GhostSamurai_APose_Dodge_R_Root_Montage.GhostSamurai_APose_Dodge_R_Root_Montage") 1.5)
                  (goto _label_3)
                  (else
                    (`self.PlayAnimMontage` (select `bool` _dodge :`false` (`KismetArrayLibrary.Array_Random` (`self.Left Sway`)) :`true` "/Game/GhostSamurai_Katana/GhostSamurai_Katana/Animation/Apose/Dodge/Root/GhostSamurai_APose_Dodge_L_Root_Montage.GhostSamurai_APose_Dodge_L_Root_Montage") 1.5)
                    (goto _label_3))))))
          (:`then_1`
            (`PlayerCameraManager.StartCameraShake` :`self` (`GameplayStatics.GetPlayerCameraManager` 0) :`ShakeClass` "/Game/Blueprints/BP_CameraShake.BP_CameraShake_C")))))))

(event `InputAction|Attack`
  (params (Key :type "Key Structure"))
  (bind _attack_int (`self.Attack Int`))
  (bind _current_attack_int (`self.Current Attack int`))
  ;[1 1 1] Attack
  (:`Pressed`
    (if (`self.Equip`)
      (if (not (or (`self.Dodge`) (`self.Attack`) (`self.Is Hit`)))
        (`|ExecutionSequence`
          (:`then_0`
            (set `self.Attack` true)
            (bind _output_get (set `self.Attack Int` (`KismetMathLibrary.RandomIntegerInRange` 0 4)))
            (if (== _output_get _current_attack_int)
              (if (== _attack_int 0)
                (bind _result (`/Engine/EditorBlueprintResources/StandardMacros.IncrementInt` _attack_int)
                  (:`  `
                    _))
                (else
                  (`/Engine/EditorBlueprintResources/StandardMacros.DecrementInt` _attack_int
                    (:`  `
                      _))))
              (set `self.Current Attack int` _result)
              (else
                (set `self.Current Attack int` _output_get)))
            (`self.PlayAnimMontage` (`|GetArrayItem` (`self.Attack Anim Montage`) _current_attack_int)))
          (:`then_1`
            (`PlayerCameraManager.StartCameraShake` :`self` (`GameplayStatics.GetPlayerCameraManager` 0) :`ShakeClass` "/Game/Blueprints/BP_CameraShake.BP_CameraShake_C")))))))

(event `Reset Attack`
  ;[1 1 1] Attack
  (set `self.Attack` false))

(event `self.ReceiveTick`
  (params (DeltaSeconds :type "Float (single-precision)"))
  (bind _target (`self.Target`))
  ;[1 1 1] Tick
  (`|ExecutionSequence`
    (:`then_0`
      (set `CharacterMovementComponent.bOrientRotationToMovement` (not (> (`KismetMathLibrary.VSize` (`self.GetVelocity`)) 0.0)) (`self.CharacterMovement`))
      (if (`self.Equip`)
        (bind (_direction _cameramovementcurve) (`Timeline|CameraMovement` :!label _label_4)
          (:`Update`
            (`SceneComponent.K2_SetRelativeLocation` (`self.Camera`) _cameramovementcurve false false)))
        (else
          (goto _label_4 :!via `Reverse`))))
    (:`then_1`
      (`self.Calcu Last Input`))
    (:`then_2`
      (if (`self.Lock`)
        (`/Engine/EditorBlueprintResources/StandardMacros.IsValid` _target
          (:`Is Valid`
            (`Controller.SetControlRotation` (`GameplayStatics.GetPlayerController` 0) (`KismetMathLibrary.RInterpTo` (`self.GetControlRotation`) (`KismetMathLibrary.MakeRotator` (.roll (`KismetMathLibrary.FindLookAtRotation` (`self.K2_GetActorLocation`) (`self.K2_GetActorLocation` _target))) (+ (.pitch (`KismetMathLibrary.FindLookAtRotation` (`self.K2_GetActorLocation`) (`self.K2_GetActorLocation` _target))) -30.0) (.yaw (`KismetMathLibrary.FindLookAtRotation` (`self.K2_GetActorLocation`) (`self.K2_GetActorLocation` _target)))) (`GameplayStatics.GetWorldDeltaSeconds`) 20.0))))))))

(event `InputAction|LockTarget`
  (params (Key :type "Key Structure"))
  (bind _targetwithdistance (`self.TargetWithDistance`))
  ;[1 1 1] Lock Target
  (:`Pressed`
    (`/Engine/EditorBlueprintResources/StandardMacros.FlipFlop`
      (:`A`
        (set `self.Lock` true)
        (`BlueprintMapLibrary.Map_Clear` _targetwithdistance)
        (bind _outactors (`GameplayStatics.GetAllActorsOfClass` "/Game/AI/BP_EnemyAI.BP_EnemyAI_C"))
        (for _array_element _outactors
          (`BlueprintMapLibrary.Map_Add` _targetwithdistance _array_element (`self.GetDistanceTo` _array_element self)))
        (bind _keys (`BlueprintMapLibrary.Map_Keys` _targetwithdistance))
        (bind _values (`BlueprintMapLibrary.Map_Values` _targetwithdistance))
        (set `self.Target` (`|GetArrayItem` _keys (`KismetMathLibrary.MinOfFloatArray` _values))))
      (:`B`
        (set `self.Lock` false)))))

(event `self.ReceiveBeginPlay`
  (bind _targetwithdistance (`self.TargetWithDistance`))
  ;[1 1 1] Event Begin Play
  (`BlueprintMapLibrary.Map_Clear` _targetwithdistance)
  (bind _outactors (`GameplayStatics.GetAllActorsOfClass` "/Game/AI/BP_EnemyAI.BP_EnemyAI_C"))
  (for _array_element _outactors
    (`BlueprintMapLibrary.Map_Add` _targetwithdistance _array_element (`self.GetDistanceTo` _array_element self)))
  (bind _keys (`BlueprintMapLibrary.Map_Keys` _targetwithdistance))
  (bind _values (`BlueprintMapLibrary.Map_Values` _targetwithdistance))
  (set `self.Target` (`|GetArrayItem` _keys (`KismetMathLibrary.MinOfFloatArray` _values))))

(event `AttackSphere`
  (bind _attackarrow (`self.AttackArrow`))
  (bind _returnvalue (`SceneComponent.K2_GetComponentLocation` _attackarrow))
  ;[1 1 1] Attack Sphere
  (bind (_outhits _returnvalue_2) (`KismetSystemLibrary.SphereTraceMulti` _returnvalue (+ _returnvalue (* (`SceneComponent.GetForwardVector` _attackarrow) 150.0)) 50.0 "TraceTypeQuery1"))
  (if _returnvalue_2
    (for _array_element _outhits
      (bind _asbp_enemy_ai (cast `/Game/AI/BP_EnemyAI` (`.HitActor` (`GameplayStatics.BreakHitResult` _array_element))))
      (`/Game/BP_WorldSettings/BPI_Damage.Damage` _asbp_enemy_ai 20.0 false))))

(event `/Game/BP_WorldSettings/BPI_Damage.Damage`
  (params (Damage :type "Float (double-precision)") (SpecialAttack :type Boolean))
  ;[1 1 1] Damage
  (set `self.Attack` false)
  (if (not (`self.Dodge`))
    (`PlayerCameraManager.StartCameraShake` :`self` (`GameplayStatics.GetPlayerCameraManager` 0) :`ShakeClass` "/Game/Blueprints/BP_CameraShake.BP_CameraShake_C" :`Scale` 0.5)
    (if SpecialAttack
      (`|ExecutionSequence`
        (:`then_0`
          (bind (_direction _ca_value _vignette_value) (`Timeline|PPTimeline` :!via `PlayFromStart`)
            (:`Update`
              (setmembers `PostProcessSettings` :`StructRef` (`CameraComponent.PostProcessSettings` (`self.Camera`)) :`SceneFringeIntensity` _ca_value :`VignetteIntensity` _vignette_value))))
        (:`then_1`
          (if (`self.Defend`)
            (`self.PlayAnimMontage` "/Game/GhostSamurai_Katana/GhostSamurai_Katana/Animation/Defense/Root/GhostSamurai_DefenseR_Broken_Root_Montage.GhostSamurai_DefenseR_Broken_Root_Montage")
            (else
              (`self.PlayAnimMontage` "/Game/GhostSamurai_Katana/GhostSamurai_Katana/Animation/Apose/Hit/Root/GhostSamurai_APose_Large_Hit_Root_Montage.GhostSamurai_APose_Large_Hit_Root_Montage")))
          (`KismetSystemLibrary.Delay` 0.5)
          (set `self.Is Hit` false :!label _label_5)))
      (else
        (`self.K2_SetActorRotation` (`KismetMathLibrary.FindLookAtRotation` (`self.K2_GetActorLocation`) (`self.K2_GetActorLocation` (`self.Target`))))
        (if (`self.Defend`)
          (`self.PlayAnimMontage` "/Game/GhostSamurai_Katana/GhostSamurai_Katana/Animation/Defense/Root/GhostSamurai_DefenseR_Hit01_Root_Montage.GhostSamurai_DefenseR_Hit01_Root_Montage")
          (`KismetSystemLibrary.Delay` 0.3)
          (goto _label_5)
          (else
            (`self.PlayAnimMontage` "/Game/GhostSamurai_Katana/GhostSamurai_Katana/Animation/Apose/Hit/Root/GhostSamurai_APose_Hit_F_Root_Montage.GhostSamurai_APose_Hit_F_Root_Montage")
            (`KismetSystemLibrary.Delay` 0.5)
            (goto _label_5)))))))

(fn `Calcu Last Input`
  (bind _returnvalue (`PawnMovementComponent.GetLastInputVector` (`self.CharacterMovement`)))
  (set `self.LastInputVector` _returnvalue)
  (bind _output_get (set `self.Input?` (!= _returnvalue (0.0 0.0 0.0) :`ErrorTolerance` 0.0001)))
  (if _output_get
    (set `self.Last Rot` (`KismetMathLibrary.MakeRotFromX` _returnvalue))))

(fn `RInterpToRot`
  (params (`Is Interp?` :type Boolean))
  (if `Is Interp?`
    (`self.K2_SetActorRotation` (`KismetMathLibrary.RInterpTo` (`self.K2_GetActorRotation`) (`self.Last Rot`) (`GameplayStatics.GetWorldDeltaSeconds`) 15.0))))

(fn `UserConstructionScript`)