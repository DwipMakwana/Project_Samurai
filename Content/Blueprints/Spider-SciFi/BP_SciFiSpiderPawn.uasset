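; A sci-fi spider character that pursues the player via AI navigation and also accepts axis input for movement.
; On BeginPlay it caches its spider Anim Blueprint and the BP_Player actor.
; Each tick it feeds its location and the player's position as a look-at target to the Anim Blueprint.
; It then starts AI MoveTo toward the player if not already moving and the player's parkour-state check passes.
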(event `InputAxis|Move Forward / Backward`
  (params (AxisValue :type "Float (single-precision)"))
  (`PawnMovementComponent.AddInputVector` (`self.CharacterMovement`) (* (`self.GetActorForwardVector`) AxisValue) false))

(event `InputAxis|Move Right / Left`
  (params (AxisValue :type "Float (single-precision)"))
  (`PawnMovementComponent.AddInputVector` (`self.CharacterMovement`) (* (`self.GetActorRightVector`) AxisValue) false))

(event `self.ReceiveBeginPlay`
  (bind _asabp_sci_fi_spider (cast `/Game/Blueprints/Spider-SciFi/ABP_SciFi_Spider` (`SkeletalMeshComponent.GetAnimInstance` (`self.Mesh`))))
  (set `self.ABP Sci Fi Spider` _asabp_sci_fi_spider)
  (bind _returnvalue (`GameplayStatics.GetActorOfClass` "/Game/Blueprints/Player/BP_Player.BP_Player_C"))
  (set `self.Player` _returnvalue))

(event `self.ReceiveTick`
  (params (DeltaSeconds :type "Float (single-precision)"))
  (bind _abp_sci_fi_spider (`self.ABP Sci Fi Spider`)
    (:`then`
      (set `/Game/Blueprints/Spider-SciFi/ABP_SciFi_Spider.ActorLocation` (`self.K2_GetActorLocation`) _abp_sci_fi_spider)
      (set `/Game/Blueprints/Spider-SciFi/ABP_SciFi_Spider.LookAt` (`self.K2_GetActorLocation` (`self.Player`)) _abp_sci_fi_spider)
      (`self.MoveToPlayer`))
    (:`else`)))

(event `MoveToPlayer`
  (if (and (not (`self.IsMoving`)) (`/Game/Blueprints/Player/BP_Player.CheckParkorState` (`self.Player`)))
    (set `self.IsMoving` true)
    (`|AIMoveTo` self (0.0 0.0 0.0) (`self.Player`) 100.0 true
      (:`OnSuccess`
        _)
      (:`OnFail`
        _))
    (set `self.IsMoving` false)))

(fn `UserConstructionScript`)